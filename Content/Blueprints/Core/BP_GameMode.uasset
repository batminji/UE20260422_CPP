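; Game mode that scatters randomized loot across the map when play begins.
; GenerateItems first caches weight totals and row names from the drop tables, though Weapon and Accessory take row names from the backpack table.
; At each data-table location it spawns a BP_ItemGroup, then makes cumulative-weight rolls for count, type and ID, rerolling duplicate weapons.
; Each result spawns its matching world item class at one of the group's random transforms and is initialized.
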(event EventBeginPlay
  (CallFunction|GenerateItems))

(event EventTick
  (params (DeltaSeconds :type Float%20%28single-precision%29)))

(fn ConstructionScript)

(fn GenerateItems
  ;[0.15 0.15 0.15 0.5] Cach Data Table
  (|CollapseGraph
    (:OutExecute
      ;[0.15 0.15 0.15 0.5] Item Group만 생성
      (bind _outrownames (DataTable|GetDataTableRowNames (Variables|Default|GetDT_ItemGroupLocation)))
      (for _array_element _outrownames
        (bind _returnvalue (Utilities|GetDataTableRow (Variables|Default|GetDT_ItemGroupLocation) _array_element)
          (:then
            (bind _returnvalue_2 (Game|SpawnActorfromClass "/Game/Blueprints/Item/BP_ItemGroup.BP_ItemGroup_C" (Math|Transform|MakeTransform (Utilities|Struct|BreakS_ItemGroupLocation _returnvalue) "0, 0, 0" "1.000000,1.000000,1.000000") "Undefined" "MultiplyWithRoot" 0 0))
            (LocalVariables|SetItemGruopRef _returnvalue_2)
            ;[0.15 0.15 0.15 0.5] 앞에서 캐싱한 정보를 넘김 -> DT 읽기 X
            (Utilities|Array|Clear (LocalVariables|GetItemTypes))
            (bind _randomcnt (CallFunction|GetRandomItemCnt (LocalVariables|GetRandomItemCntInfo)))
            (LocalVariables|SetSpawnTransforms (Default|GetRandomTransforms (LocalVariables|GetItemGruopRef) _randomcnt))
            (for _index (range 1 _randomcnt)
              ;[0.15 0.15 0.15 0.5] 이부분 다시 수정 필요
              (bind _randomtype (CallFunction|GetRandomItemType (LocalVariables|GetRandomItemTypeInfo) :!label _label))
              (if (Utilities|Enum|Equal(Enum) _randomtype "NewEnumerator0")
                (if (Utilities|Array|ContainsItem (LocalVariables|GetItemTypes) "NewEnumerator0")
                  (goto _label)
                  (else
                    (Utilities|Array|Add (LocalVariables|GetItemTypes) _randomtype)))
                (else
                  (Utilities|Array|Add (LocalVariables|GetItemTypes) _randomtype))))
            ;[0.15 0.15 0.15 0.5] Comment
            (for _array_element_2 (LocalVariables|GetItemTypes)
              (bind _outspawnitem (CallFunction|GetRandomItemID (LocalVariables|GetRandomItemIDInfo) _array_element_2))
              (Utilities|Array|Add (LocalVariables|GetSpawnItems) _outspawnitem))
            ;[0.15 0.15 0.15 0.5] Spawn
            (for (_array_element_3 _array_index) (LocalVariables|GetSpawnItems)
              (LocalVariables|SetItemType (.itemtype _array_element_3))
              (LocalVariables|SetSpawnID (.id _array_element_3))
              (bind _returnvalue_3 (Game|SpawnActorfromClass (Utilities|Select :Index (LocalVariables|GetItemType) :NewEnumerator0 "/Game/Blueprints/Item/WorldItems/BP_WorldItem_Weapon.BP_WorldItem_Weapon_C" :NewEnumerator1 "/Game/Blueprints/Item/WorldItems/BP_WorldItemWeaponAcc.BP_WorldItemWeaponAcc_C" :NewEnumerator2 "/Game/Blueprints/Item/WorldItems/BP_WorldItem_Ammo.BP_WorldItem_Ammo_C" :NewEnumerator3 "/Game/Blueprints/Item/WorldItems/BP_WorldItem_Health.BP_WorldItem_Health_C" :NewEnumerator4 "/Game/Blueprints/Item/WorldItems/BP_WorldItem_Boost.BP_WorldItem_Boost_C" :NewEnumerator5 "/Game/Blueprints/Item/WorldItems/BP_WorldItem_Helmet.BP_WorldItem_Helmet_C" :NewEnumerator6 "/Game/Blueprints/Item/WorldItems/BP_WorldItem_Vest.BP_WorldItem_Vest_C" :NewEnumerator7 "/Game/Blueprints/Item/WorldItems/BP_WorldItem_Backpack.BP_WorldItem_Backpack_C") (Utilities|Array|Get(acopy) (LocalVariables|GetSpawnTransforms) _array_index) "Undefined" "MultiplyWithRoot" 0 0))
              ;[0.15 0.15 0.15 0.5] Init
              (bind _asbp_world_item_base (Utilities|Casting|CastToBP_WorldItemBase _returnvalue_3))
              (Default|Init _asbp_world_item_base (LocalVariables|GetSpawnID) "1"))
            (Utilities|Array|Clear (LocalVariables|GetSpawnItems))))))))

(fn GetRandomItemCnt
  (params (InRandomInfo :type S%20Random%20Info%20Structure))
  (LocalVariables|SetRandomNumber (Math|Random|RandomIntegerinRange 1 (.totalpercent InRandomInfo)))
  (for _array_element (.rownames InRandomInfo)
    (bind _returnvalue (Utilities|GetDataTableRow (Variables|Default|GetDT_RandomCnt) _array_element)
      (:then
        (bind _output_get (LocalVariables|SetSumPercent (+ (LocalVariables|GetSumPercent) (.Percent (Utilities|Struct|BreakS_RandomCnt _returnvalue)))))
        (if (>= _output_get (LocalVariables|GetRandomNumber))
          (return (.Number (Utilities|Struct|BreakS_RandomCnt _returnvalue))))))))

(fn GetRandomItemType
  (params (InRandomItemTypeInfo :type S%20Random%20Info%20Structure))
  (LocalVariables|SetRandomValue (Math|Random|RandomIntegerinRange 1 (.totalpercent InRandomItemTypeInfo)))
  (for _array_element (.rownames InRandomItemTypeInfo)
    (bind _returnvalue (Utilities|GetDataTableRow (Variables|Default|GetDT_RandomType) _array_element)
      (:then
        (bind _output_get (LocalVariables|SetSumPercent (+ (LocalVariables|GetSumPercent) (.Percent (Utilities|Struct|BreakS_RandomType _returnvalue)))))
        (if (>= _output_get (LocalVariables|GetRandomValue))
          (return (.Type (Utilities|Struct|BreakS_RandomType _returnvalue))))))))

(fn GetRandomItemID
  (params (InRandomItemTypeInfos :type Map%20of%20E_ItemType%20Enums%20to%20Structs :default "NewEnumerator0") (InItemType :type E_ItemType%20Enum :default "NewEnumerator0"))
  (bind _value (Utilities|Map|Find InRandomItemTypeInfos InItemType))
  (bind (_totalpercent _rownames) (Utilities|Struct|BreakS_RandomInfo _value))
  (LocalVariables|SetRandomValue (Math|Random|RandomIntegerinRange 1 _totalpercent))
  (for _array_element _rownames
    (bind _returnvalue (Utilities|GetDataTableRow (Utilities|Select :Index InItemType :NewEnumerator0 "/Game/Blueprints/Data/DataTable/ItemGeneration/Random/DT_RandomWeapon.DT_RandomWeapon" :NewEnumerator1 "/Game/Blueprints/Data/DataTable/ItemGeneration/Random/DT_RandomAccesory.DT_RandomAccesory" :NewEnumerator2 "/Game/Blueprints/Data/DataTable/ItemGeneration/Random/DT_RandomAmmo.DT_RandomAmmo" :NewEnumerator3 "/Game/Blueprints/Data/DataTable/ItemGeneration/Random/DT_RandomHealth.DT_RandomHealth" :NewEnumerator4 "/Game/Blueprints/Data/DataTable/ItemGeneration/Random/DT_RandomBoost.DT_RandomBoost" :NewEnumerator5 "/Game/Blueprints/Data/DataTable/ItemGeneration/Random/DT_RandomHelmet.DT_RandomHelmet" :NewEnumerator6 "/Game/Blueprints/Data/DataTable/ItemGeneration/Random/DT_RandomVest.DT_RandomVest" :NewEnumerator7 "/Game/Blueprints/Data/DataTable/ItemGeneration/Random/DT_RandomBackpack.DT_RandomBackpack") _array_element)
      (:then
        (bind _output_get (LocalVariables|SetSumPercent (+ (LocalVariables|GetSumPercent) (Utilities|Struct|BreakS_RandomItem _returnvalue))))
        (if (>= _output_get (LocalVariables|GetRandomValue))
          (return (Utilities|Struct|MakeS_SpawnItem InItemType _array_element)))))))