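; BP_WorldItemWeaponAcc is a world item for weapon accessories: sights, muzzles, foregrips, mags and buttstocks.
; Init calls the parent, then looks up its ID in DT_WorldItem_WeaponAcc to set base item data, mesh, accessory type and weight.
; It applies the row's mesh rotation, then raises every type except sights by the mesh's Z bounds extent.
; GetWeight returns the stored weight.
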(event EventBeginPlay
  (|CallParentFunction) ; This node is disabled and will not be called.\nDrag off pins to build functionality.
)

(event Collision|EventActorBeginOverlap
  (params (OtherActor :type Actor%20Object%20Reference)))

(event EventTick
  (params (DeltaSeconds :type Float%20%28single-precision%29)))

(fn ConstructionScript
  (|CallParentFunction))

(fn Init
  (params (InID :type Name :default "None") (InSerialNumber :type String))
  (bind _staticmesh (Variables|Default|GetStaticMesh))
  (bind _boxextent (Collision|GetComponentBounds _staticmesh))
  (|CallParentFunction InID InSerialNumber)
  (bind _returnvalue (Utilities|GetDataTableRow "/Game/Blueprints/Data/DataTable/Item/DT_WorldItem_WeaponAcc.DT_WorldItem_WeaponAcc" (Variables|Default|GetID))
    (:then
      (CallFunction|InitWorldItemBaseData (.itemtype _returnvalue) (.itemname _returnvalue) (.uiprefix _returnvalue) (.staticmesh _returnvalue))
      (Variables|Default|SetAccType (.acctype _returnvalue))
      (Variables|Default|SetWeight (.weight _returnvalue))
      (Transformation|SetWorldRotation (Variables|Default|GetStaticMesh) (.rotationoffset _returnvalue) false false)
      ;[0.15 0.15 0.15 0.5] Comment
      (Transformation|AddActorLocalOffset (Math|Vector|MakeVector 0.0 0.0 (Utilities|Select :Index (Variables|Default|GetAccType) :NewEnumerator0 0.0 :NewEnumerator1 (.z _boxextent) :NewEnumerator2 (.z _boxextent) :NewEnumerator3 (.z _boxextent) :NewEnumerator4 (.z _boxextent))) false false))))

(fn GetWeight
  (return (Variables|Default|GetWeight)))